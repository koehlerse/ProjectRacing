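; BP_Car is a Chaos wheeled vehicle Blueprint that drives an on-screen speed and RPM display.
; On BeginPlay it creates the WBP_CarUI widget for the first player controller and caches the movement component cast to ChaosWheeledVehicleMovementComponent.
; Each Tick it pushes absolute forward speed, converted to whole km/h, and truncated engine RPM into the widget through SetUIData.
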(event EventBeginPlay
  (bind _returnvalue (UserInterface|CreateWidget "/Game/UI/Car/WBP_CarUI.WBP_CarUI_C" (Game|GetPlayerController 0)))
  (bind _output_get (Variables|Default|SetCarData _returnvalue))
  (UserInterface|Viewport|AddtoViewport _output_get 0)
  (bind _aschaos_wheeled_vehicle_movement_component (Utilities|Casting|CastToChaosWheeledVehicleMovementComponent (Variables|Default|GetVehicleMovementComponent)))
  (Variables|Default|SetChaosVehicleComponent _aschaos_wheeled_vehicle_movement_component))

(event Collision|EventActorBeginOverlap
  (params (OtherActor :type Actor%20Object%20Reference)))

(event EventTick
  (params (DeltaSeconds :type Float%20%28single-precision%29))
  (Default|SetUIData (Variables|Default|GetCarData) (Math|Float|Truncate (Math|Float|Absolute(Float) (* (Vehicle|GetForwardSpeed (Variables|Default|GetVehicleMovementComponent)) 0.036))) (Math|Float|Truncate (Class|ChaosWheeledVehicleMovementComponent|GetEngineRotationSpeed (Variables|Default|GetChaosVehicleComponent)))))

(fn ConstructionScript)